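; Rat NPC that wanders the level and can die.
; After a random delay it uses AI Move To toward a random nearby point with an attached movement sound, fades the sound when the move ends, then loops through a gate.
; Death stops movement and, if the sound component is valid, stops it, plays death and blood pool animations, and closes the gate to end wandering.
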(event Custom|Death
  (bind _returnvalue (Transformation|GetActorLocation))
  (bind (_x _y _z) (Math|Vector|BreakVector _returnvalue))
  (Class|NavMovementComponent|StopActiveMovement)
  (Utilities|IsValid (stale EventBeginPlay _returnvalue_2)
    (:Is%20Valid
      (Audio|Components|Audio|Stop (stale EventBeginPlay _returnvalue_2))
      (Components|Animation|PlayAnimation "/Game/Fantasy/Anims/NPC-RAT_Die.NPC-RAT_Die" false)
      (Development|SetHiddeninGame false false)
      (Components|Animation|PlayAnimation "/Game/Fantasy/Anims/BloodPool_Grow.BloodPool_Grow" false)
      (Utilities|FlowControl|Gate false) ; enters at Close
    )))

(event EventBeginPlay
  (bind _returnvalue (Transformation|GetActorLocation))
  (bind (_x _y _z) (Math|Vector|BreakVector _returnvalue))
  (Utilities|FlowControl|Delay (Math|Random|RandomFloatinRange 2.0 6.0) :!label _label)
  (AI|AIMoveTo self (Math|Vector|MakeVector (+ _x (Math|Random|RandomFloatinRange -1e+02 1e+02)) (+ _y (Math|Random|RandomFloatinRange -1e+02 1e+02)) _z) 0 5.0 false
    (:then
      (bind _returnvalue_2 (Audio|SpawnSoundAttached "/Game/Audio/SFX/Rat_Movement.Rat_Movement" (VehicleSound|GetRootComponent))))
    (:OnSuccess
      (Audio|Components|Audio|FadeOut _returnvalue_2 0.0 0.0 :!class /Script/Engine.AudioComponent :!label _label_2)
      (Utilities|FlowControl|Gate false
        (:Exit
          (goto _label))))
    (:OnFail
      (Class|NavMovementComponent|StopActiveMovement)
      (goto _label_2))))

(event Collision|EventActorBeginOverlap
  (params (OtherActor :type Actor%20Object%20Reference)))

(fn ConstructionScript)