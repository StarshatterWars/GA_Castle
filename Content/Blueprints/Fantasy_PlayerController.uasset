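; Player controller that drives a world-space cursor marker, Fantasy_MouseActor, under the mouse.
; It spawns the marker on BeginPlay and moves it every Tick to the complex visibility-trace hit point beneath the cursor.
; A click-to-move chain (gate, minimum-distance check against the controlled pawn, SimpleMoveToLocation) is present but never runs, so the controller issues no movement.
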(event EventTick
  (params (DeltaSeconds :type Float%20%28single-precision%29))
  (Transformation|SetActorLocation (stale EventBeginPlay _returnvalue) (.Location (Collision|BreakHitResult (.HitResult (Game|Player|GetHitResultUnderCursorbyChannel "TraceTypeQuery1" true)))) false))

(event EventBeginPlay
  (bind _returnvalue (Game|SpawnActorfromClass "/Game/Blueprints/Fantasy_MouseActor.Fantasy_MouseActor_C" (Math|Transform|MakeTransform (.Location (Collision|BreakHitResult (.HitResult (Game|Player|GetHitResultUnderCursorbyChannel "TraceTypeQuery1" true))))) false 0)))

(event Input|ActionEvents|InputActionSetDestination)

(fn ConstructionScript)